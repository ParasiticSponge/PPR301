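; BP_Board is a board actor in the shape system that prepares a dynamic material at BeginPlay.
; For every RandomShape actor, it creates a dynamic instance of NewMaterial with fixed U, V and Position parameters, then sets that shape's Board reference to None.
; A disconnected loop would apply the instance to every BP_Board mesh, so the running path never assigns the material.
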(event `self.ReceiveBeginPlay`
  ;[1 1 1] Dynamic Material
  (bind _outactors (`GameplayStatics.GetAllActorsOfClass` "/Script/PPR301.RandomShape"))
  (for _array_element _outactors
    (bind _returnvalue (`KismetMaterialLibrary.CreateDynamicMaterialInstance` "/Game/Assets/Materials/NewMaterial.NewMaterial" "DynamicMaterial"))
    (`MaterialInstanceDynamic.SetScalarParameterValue` _returnvalue "U" 0.2)
    (`MaterialInstanceDynamic.SetScalarParameterValue` _returnvalue "V" 0.6)
    (`MaterialInstanceDynamic.SetVectorParameterValue` _returnvalue "Position" (`KismetMathLibrary.MakeColor` 0.0 0.0 0.0 0.2))
    (set `RandomShape.board` null _array_element)))

(fn `UserConstructionScript`)